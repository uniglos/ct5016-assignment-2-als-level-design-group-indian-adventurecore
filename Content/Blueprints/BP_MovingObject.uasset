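; BP_MovingObject is an actor that moves back and forth along a Direction vector.
; A looping timer set on BeginPlay negates Direction every DirectionChangeTime seconds.
; Tick offsets the actor by Direction times Speed without sweeping or scaling by delta time, so movement ignores collision and depends on frame rate.
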(event Custom|DirectionChangeEvent
  (Variables|Default|SetDirection (* (Variables|Default|GetDirection) "-1.000000,-1.000000,-1.000000")))

(event EventBeginPlay
  (Utilities|Time|SetTimerbyEvent (delegate Custom|DirectionChangeEvent) (Variables|Default|GetDirectionChangeTime) true))

(event Collision|EventActorBeginOverlap
  (params (OtherActor :type Actor%20Object%20Reference)))

(event EventTick
  (params (DeltaSeconds :type Float%20%28single-precision%29))
  (Transformation|AddActorWorldOffset (* (Variables|Default|GetDirection) (Variables|Default|GetSpeed))))

(fn ConstructionScript)